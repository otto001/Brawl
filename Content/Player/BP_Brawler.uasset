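; Player brawler Blueprint that adds a few key-triggered actions and a wall-jump hook on top of inherited movement logic.
; P creates and shows the WD_Joining widget for player 0, while O adds an abortable, input-dependent ForceMovement mode.
; WallJumpStarted plays the WallJumpRotation timeline from the start, but the mesh yaw update meant to use its curve is disconnected.
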(event `Key|P`
  (params (Key :type "Key Structure" :default "AnyKey"))
  (:`Pressed`
    (bind _returnvalue (`|CreateWidget` "/Game/Widgets/Joining/WD_Joining.WD_Joining_C" (`GameplayStatics.GetPlayerController` 0)))
    (`UserWidget.AddToViewport` _returnvalue 0)))

(event `self.ReceiveTick`
  (params (DeltaSeconds :type "Float (single-precision)")))

(event `WallJumpStarted`
  (bind (_direction _cf_walljumprotation) (`Timeline|WallJumpRotation` :!via `PlayFromStart`)))

(event `Key|O`
  (params (Key :type "Key Structure" :default "AnyKey"))
  (:`Pressed`
    (set `self.ForceMovementData` (make `ForceMovementStruct` 400.0 600.0 false 0 true true))
    (`self.ChangeMovementMode` "ForceMovement" "Add")))

(fn `UserConstructionScript`)